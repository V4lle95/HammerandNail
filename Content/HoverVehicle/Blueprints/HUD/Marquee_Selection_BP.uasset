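; HUD Blueprint that provides drag-box (marquee) unit selection for the RTS pawn.
; Input start, hold and release events record mouse corners, clear any previous selection and toggle drawing.
; While dragging, DrawHUD paints a translucent blue rectangle, accumulates unique Pawns found inside it and prints their names; units are not removed as the box shrinks.
; On release, the selection is passed to RTS_Pawn through SetSelectedUnits.
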(event `self.ReceiveBeginPlay`
  (set `self.Pawn Ref` (cast `/Game/HoverVehicle/RTS_Pawn` (`GameplayStatics.GetPlayerPawn` 0) :!pure true)))

(event `/Game/HoverVehicle/Blueprints/Library/Marquee_Selection_IF.OnInputStart`
  (bind (_locationx _locationy) (`PlayerController.GetMousePosition` (`GameplayStatics.GetPlayerController` 0)))
  (if (>= (`KismetArrayLibrary.Array_LastIndex` (`self.SelectedUnits`)) 0)
    (for _ (`self.SelectedUnits`)
      (set `/Game/HoverVehicle/RTS_Pawn.is Units selected` false (`self.Pawn Ref`)))
    (`KismetArrayLibrary.Array_Clear` (`self.SelectedUnits`)))
  (bind _output_get (set `self.Click Start Location` (`KismetMathLibrary.MakeVector2D` _locationx _locationy)))
  (set `self.Holding Location` _output_get)
  (set `self.Is Drawing` true))

(event `/Game/HoverVehicle/Blueprints/Library/Marquee_Selection_IF.OnInputHold`
  (bind (_locationx _locationy) (`PlayerController.GetMousePosition` (`GameplayStatics.GetPlayerController` 0)))
  (set `self.Holding Location` (`KismetMathLibrary.MakeVector2D` _locationx _locationy)))

(event `/Game/HoverVehicle/Blueprints/Library/Marquee_Selection_IF.OnInputRelease `
  (params (HoldTime :type "Float (single-precision)"))
  (set `self.Is Drawing` false)
  (`/Game/HoverVehicle/RTS_Pawn.Set Selected Units` (`self.Pawn Ref`) (`self.SelectedUnits`)))

(event `self.ReceiveDrawHUD`
  (params (SizeX :type Integer) (SizeY :type Integer))
  (bind _selected_units (`self.Selected Units`))
  (if (`self.Is Drawing`)
    (`|ExecutionSequence`
      (:`then_0`
        (`self.Draw Marquee`)
        (bind _output_get (set `self.UnitsInSelectionArea` (`self.GetActorsInSelectionRectangle` "/Script/Engine.Pawn" (`self.Click Start Location`) (`self.Holding Location`) false)))
        (for _array_element _output_get
          (if (`KismetMathLibrary.ClassIsChildOf` (`GameplayStatics.GetObjectClass` _array_element) "/Script/Engine.Pawn")
            (bind _aspawn (cast `Pawn` _array_element))
            (set `self.Selected Units` _aspawn)
            (`KismetArrayLibrary.Array_AddUnique` (`self.SelectedUnits`) _selected_units)
            (`KismetSystemLibrary.PrintString` (`KismetSystemLibrary.GetDisplayName` _selected_units))))))))

(event `Draw Marquee`
  (bind _click_start_location (`self.Click Start Location`))
  (bind (_x _y) (`KismetMathLibrary.BreakVector2D` _click_start_location))
  (bind (_x_2 _y_2) (`KismetMathLibrary.BreakVector2D` (- (`self.Holding Location`) _click_start_location)))
  (`self.DrawRect` (struct :`R` 0.085229 :`G` 0.086275 :`B` 1.0 :`A` 0.3) _x _y _x_2 _y_2))

(fn `UserConstructionScript`)