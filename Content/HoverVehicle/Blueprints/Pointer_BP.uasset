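; World-space pointer marker whose 3D widget, when pressed, glides the player pawn to this actor's location.
; BeginPlay binds the widget's press to NewLoc, which sets Focus and lerps the pawn from its current position using CameraCurve.
; Tick repeats that move until ElapsedTime reaches CurveLength.
; Tick also orients the widget from the camera-to-pawn look-at rotation and keeps its height above the camera within clamped limits.
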(event `self.ReceiveBeginPlay`
  (bind _as3d_pointer_w (cast `/Game/HoverVehicle/Blueprints/Widget/3D_Pointer_w` (`WidgetComponent.GetUserWidgetObject` (`self.Widget`))))
  (set `self.Pointer Ref` _as3d_pointer_w)
  (add `/Game/HoverVehicle/Blueprints/Widget/3D_Pointer_w.Press` (`self.Pointer Ref`) (delegate `New Loc`)))

(event `New Loc`
  (bind _returnvalue (`GameplayStatics.GetPlayerPawn` 0))
  (set `self.Focus` true)
  (`self.K2_SetActorLocation` _returnvalue (`KismetMathLibrary.VLerp` (`self.K2_GetActorLocation` _returnvalue) (`self.K2_GetActorLocation`) (`CurveFloat.GetFloatValue` (`self.CameraCurve`) (/ (`self.ElapsedTime`) 3.0))) false false))

(event `self.ReceiveTick`
  (params (DeltaSeconds :type "Float (single-precision)"))
  (bind (_returnvalue_x _returnvalue_y) (`KismetMathLibrary.BreakVector` (`self.K2_GetActorLocation`)))
  (bind _widget (`self.Widget`))
  (bind (_returnvalue_x_2 _returnvalue_y_2 _returnvalue_z) (`KismetMathLibrary.BreakVector` (`PlayerCameraManager.GetCameraLocation` (`GameplayStatics.GetPlayerCameraManager` 0))))
  (bind (_returnvalue_roll _returnvalue_pitch _returnvalue_yaw) (`KismetMathLibrary.BreakRotator` (`KismetMathLibrary.FindLookAtRotation` (`PlayerCameraManager.GetCameraLocation` (`GameplayStatics.GetPlayerCameraManager` 0)) (`self.K2_GetActorLocation` (`GameplayStatics.GetPlayerPawn` 0)))))
  (`SceneComponent.K2_SetWorldRotation` _widget (`KismetMathLibrary.MakeRotator` _returnvalue_roll _returnvalue_pitch (- _returnvalue_yaw 90.0)) false false)
  (`SceneComponent.K2_SetWorldLocation` _widget (`KismetMathLibrary.MakeVector` _returnvalue_x _returnvalue_y (`KismetMathLibrary.FClamp` (+ _returnvalue_z 250.0) 1000.0 4500.0)) false false)
  (if (`self.Focus`)
    (`self.New Loc`)
    (bind _output_get (set `self.ElapsedTime` (+ (`GameplayStatics.GetWorldDeltaSeconds`) (`self.ElapsedTime`))))
    (if (>= _output_get (`self.CurveLength`))
      (set `self.ElapsedTime` 0.0)
      (set `self.Focus` false))))

(fn `UserConstructionScript`)