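; Base boat pawn driven by physics forces on its mesh from MoveForward and MoveRight input.
; At BeginPlay it sets center of mass and detaches an Arrow, which follows location while keeping its rotation as a fixed steering frame.
; Input pushes along the Arrow's axes and turns the mesh within clamped yaw; hitting non-simulating components adds a horizontal bounce impulse.
; An unconnected FloatingPawnMovement speed and torque alignment branch never runs.
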(event `self.ReceiveTick`
  (params (DeltaSeconds :type "Float (single-precision)"))
  (`SceneComponent.K2_SetRelativeLocation` (`self.Arrow`) (`self.K2_GetActorLocation`) false false))

(event `self.ReceiveBeginPlay`
  (`PrimitiveComponent.SetCenterOfMass` (`self.Boat Mesh Component`) (`self.Center Of Mass`) "None")
  (`SceneComponent.K2_DetachFromComponent` (`self.Arrow`) "KeepWorld" "KeepWorld" "KeepWorld" true))

(event `self.Boat Mesh Component.OnComponentHit`
  (params (HitComponent :type "PrimitiveComponent Object Reference") (OtherActor :type "Actor Object Reference") (OtherComp :type "PrimitiveComponent Object Reference") (NormalImpulse :type "Vector Structure") (Hit :type "HitResult Structure (by ref)"))
  (if (not (`SceneComponent.IsSimulatingPhysics` OtherComp "None"))
    (`PrimitiveComponent.AddImpulse` (`self.Boat Mesh Component`) (* (`KismetMathLibrary.Normal` (`KismetMathLibrary.MakeVector` (.x (`.Normal` (`GameplayStatics.BreakHitResult` Hit))) (.y (`.Normal` (`GameplayStatics.BreakHitResult` Hit))))) 200.0) "None" true)))

(event `InputAxis|MoveForward`
  (params (AxisValue :type "Float (single-precision)"))
  (bind _boat_mesh_component (`self.Boat Mesh Component`))
  (bind _boat_mesh_component_2 (`self.Boat Mesh Component`))
  (if (!= AxisValue 0.0)
    (`PrimitiveComponent.AddForce` _boat_mesh_component (* (`SceneComponent.GetForwardVector` (`self.Arrow`)) (* AxisValue (`self.Max Speed`))) "None" true)
    (`SceneComponent.K2_AddLocalRotation` _boat_mesh_component_2 (`KismetMathLibrary.MakeRotator` 0.0 0.0 (* AxisValue 2.0)) false false)
    (`SceneComponent.K2_SetRelativeRotation` _boat_mesh_component_2 (`KismetMathLibrary.MakeRotator` (.roll (`SceneComponent.RelativeRotation` _boat_mesh_component)) (.pitch (`SceneComponent.RelativeRotation` _boat_mesh_component)) (+ (`KismetMathLibrary.ClampAngle` (- (.yaw (`SceneComponent.RelativeRotation` _boat_mesh_component)) 180.0) -180.0) 180.0)) false false)))

(event `InputAxis|MoveRight`
  (params (AxisValue :type "Float (single-precision)"))
  (bind _boat_mesh_component (`self.Boat Mesh Component`))
  (if (!= AxisValue 0.0)
    (`PrimitiveComponent.AddForce` _boat_mesh_component (* (`SceneComponent.GetRightVector` (`self.Arrow`)) (* AxisValue (`self.Max Speed`))) "None" true)
    (`SceneComponent.K2_AddLocalRotation` _boat_mesh_component (`KismetMathLibrary.MakeRotator` 0.0 0.0 (* AxisValue 2.0)) false false)
    (`SceneComponent.K2_SetRelativeRotation` (`self.Boat Mesh Component`) (`KismetMathLibrary.MakeRotator` 0.0 0.0 (+ (`KismetMathLibrary.ClampAngle` (- (.yaw (`SceneComponent.RelativeRotation` (`self.Boat Mesh Component`))) 180.0) -90.0 90.0) 180.0)) false false)))

(fn `UserConstructionScript`
  (`SceneComponent.K2_SetWorldLocation` (`self.Arrow`) (`self.K2_GetActorLocation`) false false))