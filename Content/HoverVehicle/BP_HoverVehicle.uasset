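; Physics-driven hover vehicle pawn whose Cube body is steered and propelled by input axes.
; MoveRight applies torque around the up axis, while MoveForward applies force along an interpolated forward vector, scaled by a smoothed throttle (TurnRate) that is damped harder in reverse.
; Left mouse spawns a Test_Projectile at the cursor's hit location, and Tick prints both smoothed values for debugging.
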(event `InputAxis|MoveRight`
  (params (AxisValue :type "Float (single-precision)"))
  (`PrimitiveComponent.AddTorqueInDegrees` (`self.Cube`) (* (`self.GetActorUpVector`) (* AxisValue (`self.Turn Torque`))) "None" false))

(event `InputAxis|MoveForward`
  (params (AxisValue :type "Float (single-precision)"))
  (set `self.Turn Rate` (* (`KismetMathLibrary.FInterpTo` (`self.Turn Rate`) AxisValue (`GameplayStatics.GetWorldDeltaSeconds`) 5.0) (`KismetMathLibrary.SelectFloat` 0.75 0.9 (< AxisValue 0.0))))
  (set `self.Move Rate` (`KismetMathLibrary.VInterpTo` (`self.Move Rate`) (`self.GetActorForwardVector`) (`GameplayStatics.GetWorldDeltaSeconds`) 5.0))
  (`PrimitiveComponent.AddForce` (`self.Cube`) (* (`self.Move Rate`) (* (`self.Turn Rate`) (`self.Forward Force`))) "None" false))

(event `self.ReceiveTick`
  (params (DeltaSeconds :type "Float (single-precision)"))
  (`KismetSystemLibrary.PrintString` (`KismetStringLibrary.Concat_StrStr` (`KismetStringLibrary.BuildString_Double` "" "" (`self.Turn Rate`) " \n") (`KismetStringLibrary.BuildString_Vector` "" "" (`self.Move Rate`) " \n")) true true (struct :`G` 0.66 :`B` 1.0 :`A` 1.0) 1e-05))

(event `Key|LeftMouseButton`
  (params (Key :type "Key Structure"))
  (:`Pressed`
    (`|SpawnActorFromClass` "/Game/Projectiles/Blueprints/Test_Projectile.Test_Projectile_C" (`KismetMathLibrary.MakeTransform` (`.Location` (`GameplayStatics.BreakHitResult` (`PlayerController.GetHitResultUnderCursorByChannel` (`GameplayStatics.GetPlayerController` 0) "TraceTypeQuery1" true)))) "Undefined" "OverrideRootScale" null null)))

(fn `UserConstructionScript`)