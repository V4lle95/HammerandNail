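; Test projectile actor that removes instanced static mesh instances around it when its Cube component hits something.
; On hit, the Cube stops simulating physics and a ring of evenly spaced horizontal line traces fires from just above the actor, sized by Quantity and Radios.
; Traces that strike an InstancedStaticMeshComponent remove that instance.
; The construction script previews the ring with debug points at a fixed radius, independent of Radios.
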(event `self.ReceiveBeginPlay`
  (`SceneComponent.SetAbsolute` (`self.Cube`) true true true))

(event `self.Cube.OnComponentHit`
  (params (HitComponent :type "PrimitiveComponent Object Reference") (OtherActor :type "Actor Object Reference") (OtherComp :type "PrimitiveComponent Object Reference") (NormalImpulse :type "Vector Structure") (Hit :type "HitResult Structure (by ref)"))
  (bind _quantity (`self.Quantity`))
  (bind _returnvalue (+ (`self.K2_GetActorLocation`) (0.0 0.0 20.0)))
  (`PrimitiveComponent.SetSimulatePhysics` (`self.Cube`) false)
  (for _index (range 1 (+ _quantity 1))
    (bind (_outhit _returnvalue_2) (`KismetSystemLibrary.LineTraceSingle` :`Start` _returnvalue :`End` (+ (* (`KismetMathLibrary.Conv_RotatorToVector` (`KismetMathLibrary.MakeRotator` 0.0 0.0 (`KismetMathLibrary.Conv_IntToDouble` (* _index (/ 360 _quantity))))) (* (`self.radios`) 100.0)) _returnvalue) :`TraceChannel` "TraceTypeQuery1" :`DrawDebugType` "ForOneFrame"))
    (if _returnvalue_2
      (bind (_bblockinghit _binitialoverlap _time _distance _location _impactpoint _normal _impactnormal _physmat _hitactor _hitcomponent _hitbonename _hititem) (`GameplayStatics.BreakHitResult` _outhit))
      (bind _asinstanced_static_mesh_component (cast `InstancedStaticMeshComponent` _hitcomponent))
      (`InstancedStaticMeshComponent.RemoveInstance` _asinstanced_static_mesh_component _hititem))))

(fn `UserConstructionScript`
  (bind _quantity (`self.Quantity`))
  (for _index (range 1 (+ _quantity 1))
    (`KismetSystemLibrary.DrawDebugPoint` (+ (* (`KismetMathLibrary.Conv_RotatorToVector` (`KismetMathLibrary.MakeRotator` 0.0 0.0 (`KismetMathLibrary.Conv_IntToDouble` (* _index (/ 360 _quantity))))) (* 100.0 3.0)) (+ (`self.K2_GetActorLocation`) (0.0 0.0 20.0))) 4.0 (struct :`R` 1.0 :`A` 1.0) 5.0)))